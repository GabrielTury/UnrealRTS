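; Strategy game HUD that draws a drag-selection box between a start point and the mouse cursor.
; StartSelection stores the viewport-scaled mouse position and enables drawing, while StopSelection disables it.
; DrawHUD tracks the cursor and, beyond a minimum drag distance, draws an optional filled rectangle plus a four-line outline in an opaque version of the selection color.
; It only renders the box and does not select any actors.
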(event `self.ReceiveBeginPlay`
  (bind (_r _g _b) (`KismetMathLibrary.BreakColor` (`self.SelectionColor`)))
  (set `self.OutlineColor` (make `LinearColor` _r _g _b 1.0)))

(event `/Game/Gameplay/Interface/ISelection.StartSelection`
  (bind _returnvalue (`WidgetLayoutLibrary.GetMousePositionOnViewport`))
  (set `self.StartPoint` (* _returnvalue (`WidgetLayoutLibrary.GetViewportScale`)))
  (set `self.Drawing` true))

(event `/Game/Gameplay/Interface/ISelection.StopSelection`
  (set `self.Drawing` false))

(event `self.ReceiveDrawHUD`
  (params (SizeX :type Integer) (SizeY :type Integer))
  (bind (_startpoint_x _startpoint_y) (`KismetMathLibrary.BreakVector2D` (`self.StartPoint`)))
  (bind (_currentpoint_x _currentpoint_y) (`KismetMathLibrary.BreakVector2D` (`self.CurrentPoint`)))
  (if (`self.Drawing`)
    (bind _returnvalue (`WidgetLayoutLibrary.GetMousePositionOnViewport`))
    (set `self.CurrentPoint` (* _returnvalue (`WidgetLayoutLibrary.GetViewportScale`)))
    (if (> (`KismetMathLibrary.VSize2D` (- (`self.StartPoint`) (`self.CurrentPoint`))) (`self.MinBoxDistance`))
      (if (not (`self.OnlyOutline`))
        (`self.DrawRect` (`self.SelectionColor`) _startpoint_x _startpoint_y (- _currentpoint_x _startpoint_x) (- _currentpoint_y _startpoint_y)))
      (`self.DrawOutline`))))

(fn `DrawOutline`
  (bind _currentpoint_x (`KismetMathLibrary.BreakVector2D` (`self.CurrentPoint`)))
  (bind (_startpoint_x _startpoint_y) (`KismetMathLibrary.BreakVector2D` (`self.StartPoint`)))
  (bind (_currentpoint_x_2 _currentpoint_y) (`KismetMathLibrary.BreakVector2D` (`self.CurrentPoint`)))
  (bind _outlinethickness (`self.OutlineThickness`))
  (bind _startpoint_x_2 (`KismetMathLibrary.BreakVector2D` (`self.StartPoint`)))
  (bind (_currentpoint_x_3 _currentpoint_y_2) (`KismetMathLibrary.BreakVector2D` (`self.CurrentPoint`)))
  (bind (_startpoint_x_3 _startpoint_y_2) (`KismetMathLibrary.BreakVector2D` (`self.StartPoint`)))
  (bind (_currentpoint_x_4 _currentpoint_y_3) (`KismetMathLibrary.BreakVector2D` (`self.CurrentPoint`)))
  (bind (_startpoint_x_4 _startpoint_y_3) (`KismetMathLibrary.BreakVector2D` (`self.StartPoint`)))
  (`self.DrawLine` _startpoint_x_3 _startpoint_y_2 _startpoint_x_3 _currentpoint_y_3 (`self.OutlineColor`) _outlinethickness)
  (`self.DrawLine` _startpoint_x_4 _startpoint_y_3 _currentpoint_x _startpoint_y_3 (`self.OutlineColor`) _outlinethickness)
  (`self.DrawLine` _currentpoint_x_2 _currentpoint_y _currentpoint_x_2 _startpoint_y (`self.OutlineColor`) _outlinethickness)
  (`self.DrawLine` _currentpoint_x_3 _currentpoint_y_2 _startpoint_x_2 _currentpoint_y_2 (`self.OutlineColor`) _outlinethickness))

(fn `UserConstructionScript`)