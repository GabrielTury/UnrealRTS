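; PC_CameraController is a player controller for a pawn-driven camera with a visible mouse cursor and selection input.
; On possess it caches the BP_CameraPawn, and on BeginPlay it adds the Enhanced Input mapping context IM_DefaultInput.
; Movement input is scaled by CameraSpeed and passed to the pawn's MoveCamera.
; Mouse input sends start and stop selection messages to the HUD.
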(event `self.ReceivePossess`
  (params (PossessedPawn :type "Pawn Object Reference"))
  (bind _asbp_camera_pawn (cast `/Game/Gameplay/Blueprints/Camera/BP_CameraPawn` PossessedPawn))
  (set `self.PossesedPawn` _asbp_camera_pawn)
  (set `self.bShowMouseCursor` true))

(event `self.ReceiveBeginPlay`
  (`EnhancedInputSubsystemInterface.AddMappingContext` (pcsubsystem `EnhancedInputLocalPlayerSubsystem` self) "/Game/Gameplay/Input/IM_DefaultInput.IM_DefaultInput" 1 (struct)))

(event `EnhancedInput|/Game/Gameplay/Input/IA_CameraMovement`
  (params (ActionValue :type "Vector2D Structure") (ElapsedSeconds :type "Float (double-precision)") (TriggeredSeconds :type "Float (double-precision)") (InputAction :type "InputAction Object Reference" :default "/Game/Gameplay/Input/IA_CameraMovement.IA_CameraMovement"))
  (bind (_x _y) (`KismetMathLibrary.BreakVector2D` ActionValue))
  (bind _cameraspeed (`self.CameraSpeed`))
  (:`Triggered`
    (`/Game/Gameplay/Blueprints/Camera/BP_CameraPawn.MoveCamera` (`self.PossesedPawn`) (`KismetMathLibrary.MakeVector` (* _x _cameraspeed) (* _cameraspeed _y)))))

(event `EnhancedInput|/Game/Gameplay/Input/IA_MouseInput`
  (params (ActionValue :type Boolean) (ElapsedSeconds :type "Float (double-precision)") (TriggeredSeconds :type "Float (double-precision)") (InputAction :type "InputAction Object Reference" :default "/Game/Gameplay/Input/IA_MouseInput.IA_MouseInput"))
  (bind _returnvalue (`self.GetHUD`))
  (:`Triggered`
    (if ActionValue
      (message `/Game/Gameplay/Interface/ISelection.StartSelection` _returnvalue)
      (else
        (message `/Game/Gameplay/Interface/ISelection.StopSelection` _returnvalue)))))

(fn `UserConstructionScript`)